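; Base interactable actor with a widget prompt showing its icon, input icon and info text.
; The construction script sizes the interaction box from InteractableBounds, and Tick copies the icons and text into the widget every frame.
; ActorConfig shows or hides the prompt, passing movement mode and gamepad state when visible.
; ShowInfo forwards the info-key held state, and Interact pushes an "Interacted With" notification to the viewport.
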(event `self.ReceiveTick`
  (params (DeltaSeconds :type "Float (single-precision)"))
  (bind _asinteractable_widget (cast `/Game/Gameplay/UI/Widgets/InteractableWidget` (`WidgetComponent.GetUserWidgetObject` (`self.InteractWidget`)) :!pure true))
  ;[0.1302 0.1302 0.1302] Tick functionality
  (set `/Game/Gameplay/UI/Widgets/InteractableWidget.Icon` (`self.InteractableIcon`) _asinteractable_widget)
  (set `/Game/Gameplay/UI/Widgets/InteractableWidget.InputIcon` (`self.InteractableInputIcon`) _asinteractable_widget)
  (set `/Game/Gameplay/UI/Widgets/KeyWidget.InfoText` (`self.InteractableInfoText`) (`/Game/Gameplay/UI/Widgets/InteractableWidget.InfoKeyWidget` _asinteractable_widget)))

(event `Interact`
  ;[0.1302 0.1302 0.1302] Interact functionality
  (`/Game/Gameplay/Blueprints/Data/BFL_Interaction.Push Notifcation To Viewport` (make `/Game/Gameplay/Blueprints/Data/NotificationStruc` (make `SlateColor` (struct :`R` 1.0 :`G` 0.4885 :`A` 1.0)) "/Game/Gameplay/UI/Images/WidgetIcons/T_WInteract.T_WInteract" "Interacted With")))

(event `ShowInfo`
  (params (InfoKeyHeld :type Boolean))
  ;[0.1302 0.1302 0.1302] Info functionality
  (set `/Game/Gameplay/UI/Widgets/KeyWidget.IsInfoKeyHeld` InfoKeyHeld (`/Game/Gameplay/UI/Widgets/InteractableWidget.InfoKeyWidget` (cast `/Game/Gameplay/UI/Widgets/InteractableWidget` (`WidgetComponent.GetUserWidgetObject` (`self.InteractWidget`)) :!pure true))))

(fn `ActorConfig`
  (params (IconVisibility :type "/Game/Gameplay/Blueprints/Data/IconVisibiltyEnum Enum" :default "NewEnumerator0") (UsingGamepad :type Boolean) (MovementMode :type "/Game/Gameplay/Blueprints/Data/MovementModeEnum Enum" :default "NewEnumerator0"))
  (bind _asinteractable_widget (cast `/Game/Gameplay/UI/Widgets/InteractableWidget` (`WidgetComponent.GetUserWidgetObject` (`self.InteractWidget`)) :!pure true))
  ;[0.1302 0.1302 0.1302] This configuration gets used when the player can interact
  (switch `/Game/Gameplay/Blueprints/Data/IconVisibiltyEnum` IconVisibility
    (:`NewEnumerator0`
      (`/Game/Gameplay/UI/Widgets/InteractableWidget.Show` _asinteractable_widget MovementMode)
      (set `/Game/Gameplay/UI/Widgets/InteractableWidget.IsUsingGamepad` UsingGamepad _asinteractable_widget))
    (:`NewEnumerator1`
      (`/Game/Gameplay/UI/Widgets/InteractableWidget.Hide` _asinteractable_widget))))

(fn `UserConstructionScript`
  (`BoxComponent.SetBoxExtent` (`self.InteractableBox`) (`self.InteractableBounds`) true))