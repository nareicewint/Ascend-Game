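; Quest helper Blueprint that tracks a kill-all objective for actors of a given class and tag.
; Setup adds the objective to screen, registers a false flag per matching actor, and hands each actor the widget, quest and this verifier.
; Each update flips the first false flag, so kills act as a counter.
; Once the last flag is true, it updates the quest's single or multiple objective.
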(event `Update kill actors objective`
  (params (`Multiples objectives?` :type Boolean) (`quest ref` :type "/Game/Gameplay/QuestSystem/Blueprints/Quest_Base_BP/Quest_base Object Reference"))
  (bind _killed_actors (`self.Killed actors`))
  ;[0.2135 0.2135 0.2135] See if all tagged actors are killed and update the objective
  (for (_array_element _array_index) _killed_actors
    (if (not _array_element)
      (`KismetArrayLibrary.Array_Set` _killed_actors _array_index true)
      (break)))
  (if (`|GetArrayItem` _killed_actors (`KismetArrayLibrary.Array_LastIndex` _killed_actors))
    (if `Multiples objectives?`
      (`/Game/Gameplay/QuestSystem/Blueprints/Quest_Base_BP/Quest_base.Update multiples objectives` `quest ref`)
      (else
        (`/Game/Gameplay/QuestSystem/Blueprints/Quest_Base_BP/Quest_base.Update objective` `quest ref`)))))

(event `Set actors`
  (params (ActorClass :type "Actor Class Reference") (Tag :type Name) (`Multiples objectives` :type Boolean) (Text :type Text))
  (bind _quest_ref (`self.Quest ref`))
  (bind _outactors (`GameplayStatics.GetAllActorsOfClassWithTag` ActorClass Tag))
  (if `Multiples objectives`
    (bind _returnvalue (`KismetArrayLibrary.Array_Add` (`/Game/Gameplay/QuestSystem/Blueprints/Quest_Base_BP/Quest_base.Multiples Objectives` _quest_ref))))
  (bind _returnvalue_2 (`/Game/Gameplay/QuestSystem/Blueprints/Quest_Base_BP/Quest_base.Add Objective to Screen` _quest_ref Text "Visible" _returnvalue))
  (for _array_element _outactors
    (`KismetArrayLibrary.Array_Add` (`self.Killed Actors`))
    (message `/Game/Gameplay/QuestSystem/Blueprints/Quest_Base_BP/Quest_interface.Set is quest` _array_element false _returnvalue_2 `Multiples objectives` (`self.Quest ref`) self)))

(fn `UserConstructionScript`)