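; Quest location objective actor that completes an objective when the player character reaches its box trigger.
; SetIsQuest stores the owning quest, the objective widget and whether the quest has multiple objectives; in that mode, BeginPlay adds a false entry to the quest's objective list.
; On overlap by Quest_ThirdPersonCharacter, it calls the quest's single or multiple objective update, removes the widget and destroys itself.
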(event `/Game/Gameplay/QuestSystem/Blueprints/Quest_Base_BP/Quest_interface.Set is quest`
  (params (`Is quest` :type Boolean) (`Widget Objective` :type "/Game/Gameplay/QuestSystem/Blueprints/HUD/Objective_Widget Object Reference") (`Multiples objectives?` :type Boolean) (quest :type "/Game/Gameplay/QuestSystem/Blueprints/Quest_Base_BP/Quest_base Object Reference") (Kill_Actors_Verify :type "/Game/Gameplay/QuestSystem/Blueprints/Quest_Base_BP/Kill_Actors_Verify Object Reference"))
  ;[0 0 0] Set Widget
  (set `self.Widget` `Widget Objective`)
  (set `self.quest` quest)
  (set `self.Multiples objectives` `Multiples objectives?`))

(event `self.Box.OnComponentBeginOverlap`
  (params (OverlappedComponent :type "PrimitiveComponent Object Reference") (OtherActor :type "Actor Object Reference") (OtherComp :type "PrimitiveComponent Object Reference") (OtherBodyIndex :type Integer) (bFromSweep :type Boolean) (SweepResult :type "HitResult Structure (by ref)"))
  (bind _quest (`self.quest`))
  ;[0 0 0] After reach this location, the objective quest updates to the next objective
  ;;[1 0.03079 0] Change this Cast to your character
  (cast `/Game/Gameplay/QuestSystem/Blueprints/Quest_ThirdPerson_BP/Quest_ThirdPersonCharacter` OtherActor)
  (if (`self.Multiples objectives`)
    (`/Game/Gameplay/QuestSystem/Blueprints/Quest_Base_BP/Quest_base.Update multiples objectives` _quest)
    (else
      (`/Game/Gameplay/QuestSystem/Blueprints/Quest_Base_BP/Quest_base.Update objective` _quest)))
  (`Widget.RemoveFromParent` (`self.Widget`))
  (`self.K2_DestroyActor`))

(event `self.ReceiveBeginPlay`
  (if (`self.Multiples objectives`)
    (`KismetArrayLibrary.Array_Add` (`/Game/Gameplay/QuestSystem/Blueprints/Quest_Base_BP/Quest_base.Multiples Objectives` (`self.quest`)))))

(fn `UserConstructionScript`)