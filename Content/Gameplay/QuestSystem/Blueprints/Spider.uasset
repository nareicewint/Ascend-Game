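; Spider enemy that serves as a kill target for quests and chases the player on sight.
; SetIsQuest stores the quest, objective widget and kill-verify references, linking the verifier to the widget.
; Any damage destroys the spider and updates the kill objective, removing the widget when the last KilledActors entry is true.
; PawnSensing triggers AIMoveTo toward the player character.
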(event `/Game/Gameplay/QuestSystem/Blueprints/Quest_Base_BP/Quest_interface.Set is quest`
  (params (`Is quest` :type Boolean) (`Widget Objective` :type "/Game/Gameplay/QuestSystem/Blueprints/HUD/Objective_Widget Object Reference") (`Multiples objectives?` :type Boolean) (quest :type "/Game/Gameplay/QuestSystem/Blueprints/Quest_Base_BP/Quest_base Object Reference") (Kill_Actors_Verify :type "/Game/Gameplay/QuestSystem/Blueprints/Quest_Base_BP/Kill_Actors_Verify Object Reference"))
  ;[0 0 0] Sets for the current quest
  (set `self.is quest` `Is quest`)
  (bind _output_get (set `self.Widget` `Widget Objective`))
  (set `self.Multiples objectives` `Multiples objectives?`)
  (set `self.Quest` quest)
  (bind _output_get_2 (set `self.Kill_verify_ref` Kill_Actors_Verify))
  (set `/Game/Gameplay/QuestSystem/Blueprints/HUD/Objective_Widget.Kill_Verify_ref` _output_get_2 _output_get))

(event `self.ReceiveAnyDamage`
  (params (Damage :type "Float (single-precision)") (DamageType :type "DamageType Object Reference") (InstigatedBy :type "Controller Object Reference") (DamageCauser :type "Actor Object Reference"))
  (bind _killed_actors (`/Game/Gameplay/QuestSystem/Blueprints/Quest_Base_BP/Kill_Actors_Verify.Killed Actors` (`self.Kill_verify_ref`)))
  ;[0 0 0] When receive damage die
  (`|ExecutionSequence`
    (:`then_0`
      (`self.K2_DestroyActor`))
    (:`then_1`
      (`/Game/Gameplay/QuestSystem/Blueprints/Quest_Base_BP/Kill_Actors_Verify.Update kill actors objective` (`self.Kill_verify_ref`) (`self.Multiples objectives`) (`self.Quest`))
      (if (`|GetArrayItem` _killed_actors (`KismetArrayLibrary.Array_LastIndex` _killed_actors))
        (`Widget.RemoveFromParent` (`self.Widget`))))))

(event `self.PawnSensing.OnSeePawn`
  (params (Pawn :type "Pawn Object Reference"))
  ;[0 0 0] When the player is in line of sight, go to him
  (bind _asquest_third_person_character (cast `/Game/Gameplay/QuestSystem/Blueprints/Quest_ThirdPerson_BP/Quest_ThirdPersonCharacter` Pawn))
  (if (== Pawn _asquest_third_person_character)
    (`|AIMoveTo` self (`self.K2_GetActorLocation` _asquest_third_person_character) _asquest_third_person_character 100.0)))

(fn `UserConstructionScript`)