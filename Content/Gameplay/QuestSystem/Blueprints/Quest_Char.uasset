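; Interactable quest character that shows a brief greeting and can complete quest objectives.
; Its sphere overlap registers or clears it as the player character's ActorToInteract.
; SetIsQuest stores the quest, objective widget and multi-objective flag.
; Interact flashes Hello and, when flagged, clears the flag, removes the widget, updates single or multiple objectives, then calls SetIsQuestMessage on the current quest's ActorsToInteract.
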(event `/Game/Gameplay/QuestSystem/Blueprints/Quest_Base_BP/Quest_interface.Set is quest`
  (params (`Is quest` :type Boolean) (`Widget Objective` :type "/Game/Gameplay/QuestSystem/Blueprints/HUD/Objective_Widget Object Reference") (`Multiples objectives?` :type Boolean) (quest :type "/Game/Gameplay/QuestSystem/Blueprints/Quest_Base_BP/Quest_base Object Reference") (Kill_Actors_Verify :type "/Game/Gameplay/QuestSystem/Blueprints/Quest_Base_BP/Kill_Actors_Verify Object Reference"))
  ;[0 0 0] Set that it's part of the current quest
  (set `self.Is quest` `Is quest`)
  (set `self.Widget` `Widget Objective`)
  (set `self.Quest` quest)
  (set `self.Multiples objectives` `Multiples objectives?`))

(event `/Game/Gameplay/QuestSystem/Blueprints/Quest_Base_BP/Quest_interface.Interact`
  (bind _hello (`self.hello`))
  (bind _quest (`self.Quest`))
  ;[0 0 0 1 30] Interact
  (`|ExecutionSequence`
    (:`then_0`
      ;;[0.2314 0.2314 0.2314] Custom Dialog Interaction
      (`SceneComponent.SetVisibility` _hello true false)
      (`KismetSystemLibrary.Delay` 2.0)
      (`SceneComponent.SetVisibility` _hello false false))
    (:`then_1`
      ;;[0.2314 0.2314 0.2314 1 22] Update Quest
      (if (`self.Is quest`)
        ;;;[1 0.03079 0] Change this Cast to your character
        (bind _asquest_third_person_character (cast `/Game/Gameplay/QuestSystem/Blueprints/Quest_ThirdPerson_BP/Quest_ThirdPersonCharacter` (`GameplayStatics.GetPlayerCharacter` 0)))
        (set `self.Is quest` false)
        (`Widget.RemoveFromParent` (`self.Widget`))
        (if (`self.Multiples objectives`)
          (`/Game/Gameplay/QuestSystem/Blueprints/Quest_Base_BP/Quest_base.Update multiples objectives` _quest)
          (set `self.Multiples objectives` false)
          (else
            (`/Game/Gameplay/QuestSystem/Blueprints/Quest_Base_BP/Quest_base.Update objective` _quest)))
        (for _array_element (`/Game/Gameplay/QuestSystem/Blueprints/Quest_Base_BP/Quest_base.Actors to interact` (`/Game/Gameplay/QuestSystem/Blueprints/Quest_ThirdPerson_BP/Quest_ThirdPersonCharacter.Current_quest` _asquest_third_person_character))
          (message `/Game/Gameplay/QuestSystem/Blueprints/Quest_Base_BP/Quest_interface.Set is quest` _array_element false null false null null))))))

(event `self.Sphere.OnComponentBeginOverlap`
  (params (OverlappedComponent :type "PrimitiveComponent Object Reference") (OtherActor :type "Actor Object Reference") (OtherComp :type "PrimitiveComponent Object Reference") (OtherBodyIndex :type Integer) (bFromSweep :type Boolean) (SweepResult :type "HitResult Structure (by ref)"))
  ;[0 0 0] Define actor that the player can interact
  ;;[1 0.03079 0] Change this Cast to your character
  (bind _asquest_third_person_character (cast `/Game/Gameplay/QuestSystem/Blueprints/Quest_ThirdPerson_BP/Quest_ThirdPersonCharacter` OtherActor))
  (set `/Game/Gameplay/QuestSystem/Blueprints/Quest_ThirdPerson_BP/Quest_ThirdPersonCharacter.Actor to interact` self _asquest_third_person_character))

(event `self.Sphere.OnComponentEndOverlap`
  (params (OverlappedComponent :type "PrimitiveComponent Object Reference") (OtherActor :type "Actor Object Reference") (OtherComp :type "PrimitiveComponent Object Reference") (OtherBodyIndex :type Integer))
  ;[0 0 0] Define actor that the player can interact
  ;;[1 0.03079 0] Change this Cast to your character
  (bind _asquest_third_person_character (cast `/Game/Gameplay/QuestSystem/Blueprints/Quest_ThirdPerson_BP/Quest_ThirdPersonCharacter` OtherActor))
  (set `/Game/Gameplay/QuestSystem/Blueprints/Quest_ThirdPerson_BP/Quest_ThirdPersonCharacter.Actor to interact` null _asquest_third_person_character))

(fn `UserConstructionScript`)