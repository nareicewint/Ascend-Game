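; A linear quest Blueprint that walks the player through three sequential interaction objectives, then pays out a reward.
; The NextObjective event switches on the step index, calling InteractObjective with a target class, tag, actor names and objective text.
; The steps are talking to any of three characters, interacting with a pink cube, and collecting from a green character.
; The last step calls FinalizeQuest with money, item entries at zero quantity, and itself as NextQuest.
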(event `self.Next Objective`
  (params (Int :type Integer))
  (switch `int` Int
    (:`0`
      (`self.Interact objective` "/Game/Gameplay/QuestSystem/Blueprints/Quest_Char.Quest_Char_C" "anyone" (`|MakeArray` "character 2" "character 3" "character 4") false "Talk to anyone of the three guys at center of map."))
    (:`1`
      (`self.Interact objective` "/Game/Gameplay/QuestSystem/Blueprints/Quest_Object.Quest_Object_C" "interact" (`|MakeArray` "Cube") false "Interact with the pink cube."))
    (:`2`
      (`self.Interact objective` "/Game/Gameplay/QuestSystem/Blueprints/Quest_Char.Quest_Char_C" "green" (`|MakeArray` "character 5") false "Take your reward with Green guy!"))
    (:`3`
      (`self.Finalize Quest` "NewEnumerator0" 200.0 (`|MakeArray` "NewEnumerator0" "NewEnumerator2" :!type "/Game/Gameplay/QuestSystem/Blueprints/Quest_Base_BP/Item Enum") (`|MakeArray` 0 0) "3_Linear_Quest_C"))))

(fn `UserConstructionScript`
  (`parent.UserConstructionScript`))