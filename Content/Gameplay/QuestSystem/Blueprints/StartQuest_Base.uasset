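; Base interactable quest-starter actor that gives the player a quest and can also serve as a quest objective.
; Box overlap sets or clears it as the Quest_ThirdPersonCharacter's ActorToInteract.
; Interact spawns the Quest class once (re-armed by Reset_Once), adds it to AcceptedQuests, making it current if none is.
; When flagged through SetIsQuest, Interact also removes the objective widget and updates the referenced quest's single or multiple objectives.
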(event `self.Box.OnComponentBeginOverlap`
  (params (OverlappedComponent :type "PrimitiveComponent Object Reference") (OtherActor :type "Actor Object Reference") (OtherComp :type "PrimitiveComponent Object Reference") (OtherBodyIndex :type Integer) (bFromSweep :type Boolean) (SweepResult :type "HitResult Structure (by ref)"))
  ;[0 0 0] Define Actor That The Player Can Interact
  ;;[1 0.03079 0] Change this Cast to your character
  (bind _asquest_third_person_character (cast `/Game/Gameplay/QuestSystem/Blueprints/Quest_ThirdPerson_BP/Quest_ThirdPersonCharacter` OtherActor))
  (set `/Game/Gameplay/QuestSystem/Blueprints/Quest_ThirdPerson_BP/Quest_ThirdPersonCharacter.Actor to interact` self _asquest_third_person_character))

(event `self.Box.OnComponentEndOverlap`
  (params (OverlappedComponent :type "PrimitiveComponent Object Reference") (OtherActor :type "Actor Object Reference") (OtherComp :type "PrimitiveComponent Object Reference") (OtherBodyIndex :type Integer))
  ;[0 0 0] Define Actor That The Player Can Interact
  ;;[1 0.03079 0] Change this Cast to your character
  (bind _asquest_third_person_character (cast `/Game/Gameplay/QuestSystem/Blueprints/Quest_ThirdPerson_BP/Quest_ThirdPersonCharacter` OtherActor))
  (set `/Game/Gameplay/QuestSystem/Blueprints/Quest_ThirdPerson_BP/Quest_ThirdPersonCharacter.Actor to interact` null _asquest_third_person_character))

(event `/Game/Gameplay/QuestSystem/Blueprints/Quest_Base_BP/Quest_interface.Interact`
  (bind _quest (`self.quest`))
  (bind _quest_ref (`self.Quest_ref`))
  ;[0 0 0] Activate Quest
  (`|ExecutionSequence`
    (:`then_0`
      (`/Engine/EditorBlueprintResources/StandardMacros.DoOnce` false :!label _label
        (:`Completed`
          ;;[1 0.03079 0] Change this Cast to your character
          (bind _asquest_third_person_character (cast `/Game/Gameplay/QuestSystem/Blueprints/Quest_ThirdPerson_BP/Quest_ThirdPersonCharacter` (`GameplayStatics.GetPlayerCharacter` 0)))
          (if (`KismetSystemLibrary.IsValidClass` _quest)
            (bind _returnvalue (`|SpawnActorFromClass` _quest (`KismetMathLibrary.MakeTransform` (0.0 0.0 0.0)) "Undefined" "OverrideRootScale" null null))
            (`/Engine/EditorBlueprintResources/StandardMacros.IsValid` (`/Game/Gameplay/QuestSystem/Blueprints/Quest_ThirdPerson_BP/Quest_ThirdPersonCharacter.Current_quest` _asquest_third_person_character)
              (:`Is Valid`
                (bind _accepted_quests (`/Game/Gameplay/QuestSystem/Blueprints/Quest_ThirdPerson_BP/Quest_ThirdPersonCharacter.Accepted_quests` _asquest_third_person_character))
                (`KismetArrayLibrary.Array_Add` _accepted_quests _returnvalue))
              (:`Is Not Valid`
                (bind _output_get (set `/Game/Gameplay/QuestSystem/Blueprints/Quest_ThirdPerson_BP/Quest_ThirdPersonCharacter.Current_quest` _returnvalue _asquest_third_person_character))
                (`KismetArrayLibrary.Array_Add` _accepted_quests _output_get)))
            (set `/Game/Gameplay/QuestSystem/Blueprints/Quest_Base_BP/Quest_base.quest starter` self _returnvalue)
            (`/Game/Gameplay/QuestSystem/Blueprints/Quest_ThirdPerson_BP/Quest_ThirdPersonCharacter.Show_quests` _asquest_third_person_character)))))
    (:`then_1`
      ;[0 0 0 1 30] Interact
      ;;[0.2314 0.2314 0.2314 1 22] Update Quest
      (if (`self.Is quest`)
        ;;;[1 0.03079 0] Change this Cast to your character
        (cast `/Game/Gameplay/QuestSystem/Blueprints/Quest_ThirdPerson_BP/Quest_ThirdPersonCharacter` (`GameplayStatics.GetPlayerCharacter` 0))
        (set `self.Is quest` false)
        (`Widget.RemoveFromParent` (`self.Widget`))
        (if (`self.Multiples objectives`)
          (`/Game/Gameplay/QuestSystem/Blueprints/Quest_Base_BP/Quest_base.Update multiples objectives` _quest_ref)
          (set `self.Multiples objectives` false)
          (else
            (`/Game/Gameplay/QuestSystem/Blueprints/Quest_Base_BP/Quest_base.Update objective` _quest_ref)))))))

(event `Reset_Once`
  ;[0 0 0] Activate Quest
  (goto _label :!via `Reset`))

(event `/Game/Gameplay/QuestSystem/Blueprints/Quest_Base_BP/Quest_interface.Set is quest`
  (params (`Is quest` :type Boolean) (`Widget Objective` :type "/Game/Gameplay/QuestSystem/Blueprints/HUD/Objective_Widget Object Reference") (`Multiples objectives?` :type Boolean) (quest :type "/Game/Gameplay/QuestSystem/Blueprints/Quest_Base_BP/Quest_base Object Reference") (Kill_Actors_Verify :type "/Game/Gameplay/QuestSystem/Blueprints/Quest_Base_BP/Kill_Actors_Verify Object Reference"))
  ;[0 0 0] Set that it's part of the current quest
  (set `self.Is quest` `Is quest`)
  (set `self.Widget` `Widget Objective`)
  (set `self.Quest_ref` quest)
  (set `self.Multiples objectives` `Multiples objectives?`))

(fn `UserConstructionScript`)