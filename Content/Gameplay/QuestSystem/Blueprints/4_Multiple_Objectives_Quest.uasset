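; Quest Blueprint that demonstrates simultaneous objectives: killing red and white spiders, then returning for a reward.
; A NextObjective event switches on the step index, first spawning tagged spiders and registering both kill objectives as multiple objectives.
; It then sets an interact objective on the quest giver Start_quest4.
; The last step finalizes the quest with item rewards and names this same quest as the next one.
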(event `self.Next Objective`
  (params (Int :type Integer))
  (switch `int` Int
    (:`0`
      (`self.Spawn actors to kill` "/Game/Gameplay/QuestSystem/Blueprints/Red_Spider.Red_Spider_C" (-520.0 1030.0 200.0) (6.0 6.0 6.0) "red spider" 1)
      (`self.Spawn actors to kill` "/Game/Gameplay/QuestSystem/Blueprints/Spider.Spider_C" (-1320.0 1030.0 200.0) (6.0 6.0 6.0) "spider")
      (`self.Kill actors objective` "/Game/Gameplay/QuestSystem/Blueprints/Red_Spider.Red_Spider_C" "red spider" true "Kill 2 Red spiders")
      (`self.Kill actors objective` "/Game/Gameplay/QuestSystem/Blueprints/Spider.Spider_C" "spider" true "Kill 1 white spider"))
    (:`1`
      (`self.Interact objective` "/Game/Gameplay/QuestSystem/Blueprints/StartQuest_Base.StartQuest_Base_C" "reward" (`|MakeArray` "Start_quest4") false "Back and take the reward"))
    (:`2`
      (`self.Finalize Quest` "NewEnumerator1" 0.0 (`|MakeArray` "NewEnumerator0" "NewEnumerator2" :!type "/Game/Gameplay/QuestSystem/Blueprints/Quest_Base_BP/Item Enum") (`|MakeArray` 3 5) "4_Multiple_Objectives_Quest_C"))))

(fn `UserConstructionScript`
  (`parent.UserConstructionScript`))