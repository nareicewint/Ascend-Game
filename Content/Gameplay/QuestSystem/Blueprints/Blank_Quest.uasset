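; Blank template Blueprint for authoring a new quest in the quest system.
; The NextObjective event switches on an objective index, but no cases are wired yet.
; Unconnected example nodes show the available building blocks: interact, location and kill objectives, spawning actors to kill, and finalizing the quest with item and quantity arrays.
; The construction script only calls its parent.
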(event `self.Next Objective`
  (params (Int :type Integer))
  (switch `int` Int))

(fn `UserConstructionScript`
  (`parent.UserConstructionScript`))