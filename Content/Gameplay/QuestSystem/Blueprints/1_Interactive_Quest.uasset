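; Quest Blueprint for an interactive objective that sends the player to talk with the Red Guy character.
; NextObjective switches on the step index, calling InteractObjective to target a Quest_Char tagged "red" on the first and third steps.
; The middle step calls FinalizeQuest with money and item rewards, naming this same quest as the next one, then calls UpdateObjective.
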(event `self.Next Objective`
  (params (Int :type Integer))
  (switch `int` Int
    (:`0`
      (`self.Interact objective` "/Game/Gameplay/QuestSystem/Blueprints/Quest_Char.Quest_Char_C" "red" (`|MakeArray` "character 1") false "Go talk with Red Guy!"))
    (:`1`
      (`self.Finalize Quest` "NewEnumerator2" 10.0 (`|MakeArray` "NewEnumerator0" "NewEnumerator2" :!type "/Game/Gameplay/QuestSystem/Blueprints/Quest_Base_BP/Item Enum") (`|MakeArray` 1 1) "1_Interactive_Quest_C")
      (`self.Update objective`))
    (:`2`
      (`self.Interact objective` "/Game/Gameplay/QuestSystem/Blueprints/Quest_Char.Quest_Char_C" "red" (`|MakeArray` "character 1") false "Go talk with Red Guy!"))))

(fn `UserConstructionScript`
  (`parent.UserConstructionScript`))